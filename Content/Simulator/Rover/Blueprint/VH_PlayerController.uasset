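; Player controller for the rover simulator that tracks laps and lap times from vehicle overlap events.
; Checkpoint overlaps flag points A, B and C by actor display name and notify the HUD.
; A FinishLine trigger overlap with all three flags set counts a lap and resets them.
; Lap time comes from the game state's total time minus prior cumulative time, updating the best lap and HUD.
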(event `Event VH OverlapUpdate (Controller)`
  (params (Actor :type "Actor Object Reference"))
  (bind _bestlaptime (`self.BestLapTime`))
  (bind _laptime (`self.LapTime`))
  ;[1 1 1] Lap Tracking setup
  (bind _asvehicle_track_point (cast `VehicleTrackPoint` Actor)
    (:`then`
      (bind _asvh_hud (cast `/Game/Simulator/Rover/Blueprint/VH_HUD` (`self.GetHUD`)))
      (`/Game/Simulator/Rover/Blueprint/VH_HUD.Event DisplayCheckpoint (HUD)` _asvh_hud)
      (bind _returnvalue (`KismetSystemLibrary.GetDisplayName` _asvehicle_track_point))
      (if (`KismetStringLibrary.EqualEqual_StrStr` _returnvalue "CheckPointA")
        (set `self.PointA` true)
        (elif (`KismetStringLibrary.EqualEqual_StrStr` _returnvalue "CheckPointB")
          (set `self.PointB` true)
          (elif (`KismetStringLibrary.EqualEqual_StrStr` _returnvalue "CheckPointC")
            (set `self.PointC` true)))))
    (:`CastFailed`
      (bind _astrigger_box (cast `TriggerBox` Actor))
      (if (`KismetStringLibrary.EqualEqual_StrStr` (`KismetSystemLibrary.GetDisplayName` _astrigger_box) "FinishLine")
        (if (`self.PointA`)
          (if (`self.PointB`)
            (if (`self.PointC`)
              ;[1 1 1] Complete Another Lap
              (set `self.LapsTotal` (+ (`self.LapsTotal`) 1))
              (set `self.PointA` false)
              (set `self.PointB` false)
              (set `self.PointC` false)
              (bind _asvehicle_game_state (cast `VehicleGameState` (`GameplayStatics.GetGameState`)))
              (bind _returnvalue_2 (`VehicleGameState.GetTotalTime` _asvehicle_game_state))
              (bind _returnvalue_3 (- _returnvalue_2 (`self.CumulativeLapTime`)))
              (set `self.LapTime` _returnvalue_3)
              (`KismetArrayLibrary.Array_Add` (`self.LapTimes`) _returnvalue_3)
              (if (== _bestlaptime 0.0)
                (set `self.BestLapTime` _laptime :!label _label)
                (else
                  (`/Engine/EditorBlueprintResources/StandardMacros.CompareFloat` (`self.LapTime`) _bestlaptime
                    (:`>`
                      _)
                    (:`==`
                      _)
                    (:`<`
                      (goto _label)))))
              (set `self.CumulativeLapTime` (+ _laptime (`self.CumulativeLapTime`)))
              (bind _asvh_hud_2 (cast `/Game/Simulator/Rover/Blueprint/VH_HUD` (`self.GetHUD`)))
              (`/Game/Simulator/Rover/Blueprint/VH_HUD.Event OnLapCompleted (HUD)` _asvh_hud_2 (`self.LapsTotal`) (`self.BestLapTime`) (`self.CumulativeLapTime`)))))))))

(fn `UserConstructionScript`)