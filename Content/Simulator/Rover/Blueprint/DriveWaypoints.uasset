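; Waypoint sequencing function for the rover simulator that picks which point in a list the vehicle drives to next.
; It advances the index once the actor is within MaxDistance of the current waypoint, using -1 for start and -2 for finished, with Loop selecting restart or stop at the end.
; It returns the index, target and a DoMove flag that is true only when a new waypoint is selected.
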(fn `driveWaypoints`
  (params (_WayPoints :type "Array of Vector Structure") (_IndexVH :type Integer) (_loop :type Boolean) (_ActorLocation :type "Vector Structure") (_maxDistance :type "Float (double-precision)"))
  (returns (indexOut :type Integer) (moveOut :type "Vector Structure") (doMoveOut :type Boolean))
  (locals (wayPoints :type "Array of Vector Structure") (indexVH :type Integer) (loop :type Boolean) (maxDistance :type "Float (double-precision)") (doMove :type Boolean) (wayPoint :type "Vector Structure") (ActorLocation :type "Vector Structure") (currentDistance :type "Float (double-precision)"))
  (bind _item (`KismetArrayLibrary.Array_Get` (`local.wayPoints`) (`local.indexVH`)))
  (bind _returnvalue (`KismetMathLibrary.VSize` (- (`local.ActorLocation`) (`KismetArrayLibrary.Array_Get` (`local.wayPoints`) (`local.indexVH`)))))
  ;[1 1 1] Simulate Vehicle
  (set `local.wayPoints` _WayPoints)
  (set `local.indexVH` _IndexVH)
  (set `local.loop` _loop)
  (set `local.ActorLocation` _ActorLocation)
  (set `local.maxDistance` _maxDistance)
  (set `local.doMove` false)
  (if (!= (`local.indexVH`) -2)
    (if (== (`local.indexVH`) -1)
      (bind _output_get (set `local.indexVH` 0))
      (set `local.wayPoint` (`KismetArrayLibrary.Array_Get` (`local.wayPoints`) _output_get))
      (bind _output_get_2 (set `local.doMove` true))
      (`KismetSystemLibrary.PrintString` null (`KismetStringLibrary.Conv_BoolToString` _output_get_2) false false)
      (else
        (bind _output_get_3 (set `local.currentDistance` _returnvalue))
        (`KismetSystemLibrary.PrintString` null (`KismetStringLibrary.Concat_StrStr` (`KismetStringLibrary.Conv_IntToString` (`local.indexVH`)) ": " (`KismetStringLibrary.Conv_DoubleToString` _output_get_3)) false false (struct :`G` 0.66 :`B` 1.0 :`A` 1.0) 0.0)
        (if (<= _returnvalue (`local.maxDistance`))
          (set `local.indexVH` (+ (`local.indexVH`) 1))
          (if (> (`KismetArrayLibrary.Array_Length` (`local.wayPoints`)) (`local.indexVH`))
            (set `local.wayPoint` _item)
            (set `local.doMove` true)
            (elif (`local.loop`)
              (set `local.indexVH` -1)
              (else
                (set `local.indexVH` -2))))
          (else
            (set `local.wayPoint` _item))))))
  (return (`local.indexVH`) (`local.wayPoint`) (`local.doMove`)))