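; AI rover buggy vehicle that drives a looping waypoint route when StartAi is set, otherwise applying its Steering and Thrust variables.
; Tick gets the next point from DriveWaypoints and passes it to MoveToLocation, which starts a looping UpdateMovement timer.
; UpdateMovement steers from yaw error and gates full throttle by MaxSpeed.
; Within arrival range it clears the timer, fires move-completed and handbrakes unless RollingStop is set.
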(event `self.ReceiveTick`
  (params (DeltaSeconds :type "Float (single-precision)"))
  (if (`self.StartAi`)
    ;[1 1 1] WayPoint Planner
    (if (`self.StartAi`)
      (`|ExecutionSequence`
        (:`then_1`
          (bind (_indexout _moveout _domoveout) (`/Game/Simulator/Rover/Blueprint/DriveWaypoints.driveWaypoints` (`self.Waypoints`) (`self.indexVH`) true (`SceneComponent.K2_GetComponentLocation` (`self.Mesh`)) 1000.0))
          (set `self.indexVH` _indexout)
          (if _domoveout
            (`self.MoveToLocation` _moveout true)))))
    (else
      (`|ExecutionSequence`
        (:`then_0`
          ;[1 1 1] Steering input
          (`WheeledVehicleMovementComponent.SetSteeringInput` (`self.VehicleMovement`) (`self.steering`)))
        (:`then_1`
          ;[1 1 1] Throttle input
          (bind _returnvalue (`PrimitiveComponent.GetPhysicsLinearVelocity` (`self.Mesh`) "None"))
          (`WheeledVehicleMovementComponent.SetThrottleInput` (`self.VehicleMovement`) (`KismetMathLibrary.SelectFloat` (`self.thrust`) 0.0 (> (- (`self.MaxSpeed`) (`KismetMathLibrary.Dot_VectorVector` _returnvalue (`KismetMathLibrary.GetForwardVector` (`self.K2_GetActorRotation`)))) 0.0))))))))

(fn `MoveToLocation`
  (params (Location :type "Vector Structure") (`Rolling Stop` :type Boolean))
  (set `self.RollingStop` `Rolling Stop`)
  (set `self.Destination` Location)
  (set `self.Distance` (`KismetMathLibrary.VSize` (- (`self.K2_GetActorLocation`) Location)))
  (set `self.Started` (`KismetSystemLibrary.GetGameTimeInSeconds`))
  (`KismetSystemLibrary.K2_SetTimer` null "UpdateMovement" 0.03 true))

(fn `UpdateMovement`
  (locals (HoldTurn :type Boolean) (Turn :type "Float (double-precision)"))
  (bind _returnvalue (`self.K2_GetActorLocation`))
  (bind _destination (`self.Destination`))
  (bind _vehiclemovement (`self.VehicleMovement`))
  (bind _yaw (.yaw (`KismetMathLibrary.NormalizedDeltaRotator` (`KismetMathLibrary.FindLookAtRotation` _returnvalue _destination) (`self.K2_GetActorRotation`))))
  (bind _returnvalue_2 (`KismetMathLibrary.MapRangeUnclamped` _yaw -180.0 180.0 -1.0 1.0))
  (bind _returnvalue_3 (`KismetMathLibrary.InRange_FloatFloat` _yaw -90.0 90.0))
  (bind _returnvalue_4 (`KismetMathLibrary.SelectFloat` _returnvalue_2 0.0 _returnvalue_3))
  ;[1 1 1] Calculate Speed with Limit
  (`WheeledVehicleMovementComponent.SetSteeringInput` _vehiclemovement (`KismetMathLibrary.SelectFloat` -1.0 (`KismetMathLibrary.SelectFloat` _returnvalue_4 _returnvalue_2 (and (not _returnvalue_3) (< (`KismetMathLibrary.VSize` (- _returnvalue _destination)) 1000.0))) (== _returnvalue_4 0.0))) ; Update Steering Accordingly
  (bind _returnvalue_5 (`PrimitiveComponent.GetPhysicsLinearVelocity` (`self.Mesh`) "None"))
  (`WheeledVehicleMovementComponent.SetThrottleInput` _vehiclemovement (`KismetMathLibrary.SelectFloat` 1.0 0.0 (> (- (`self.MaxSpeed`) (`KismetMathLibrary.Dot_VectorVector` _returnvalue_5 (`KismetMathLibrary.GetForwardVector` (`self.K2_GetActorRotation`)))) 0.0))) ; Update Throttle Accordingly
  ;[1 1 1] Condition met sets break and clears movement state
  (if (< (`KismetMathLibrary.VSize` (- _returnvalue _destination)) 1000.0)
    (if (not (`self.RollingStop`))
      (`WheeledVehicleMovementComponent.SetHandbrakeInput` (`self.VehicleMovement`) true))
    ;[1 1 1] End Update Movement & Set States
    (set `self.State` "NewEnumerator0")
    (`self.MoveCompleted`)
    (`KismetSystemLibrary.K2_SetTimer` null "UpdateMovement")
    (set `self.State` "NewEnumerator0")
    (else
      (set `self.State` "NewEnumerator0"))))

(fn `UserConstructionScript`)