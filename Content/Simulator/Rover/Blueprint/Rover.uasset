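; Simulator rover Blueprint that passes player gas and steer input, or logged stick values, to a Rover object as thrust and steering.
; The startTarget action loads waypoints from a file and starts the rover's AI.
; While input is inactive, Tick replays one log entry per frame, then restores player control at the end.
; The nodes that load the log from a hardcoded directory and start replay are disconnected.
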(event `InputAction|startTarget`
  (params (Key :type "Key Structure" :default "AnyKey"))
  (bind _rover (`self.rover`))
  (:`Pressed`
    (bind _returnvalue (`SimulatorFunctions.readWayPoints` (`self.WaypointFile`)))
    (set `/Game/Simulator/Rover/Blueprint/AIBuggyVH.Waypoints` _returnvalue _rover)
    (set `/Game/Simulator/Rover/Blueprint/AIBuggyVH.StartAi` true _rover)))

(event `InputAxis|Gas`
  (params (AxisValue :type "Float (single-precision)"))
  (if (`self.inputActive`)
    (set `/Game/Simulator/Rover/Blueprint/AIBuggyVH.thrust` AxisValue (`self.rover`))))

(event `InputAxis|Steer`
  (params (AxisValue :type "Float (single-precision)"))
  (if (`self.inputActive`)
    (set `/Game/Simulator/Rover/Blueprint/AIBuggyVH.steering` AxisValue (`self.rover`))))

(event `self.ReceiveTick`
  (params (DeltaSeconds :type "Float (single-precision)"))
  (bind (_item_uavpos _item_uavrot _item_uavvel _item_leftstickx _item_leftsticky) (break `lightLog` (`KismetArrayLibrary.Array_Get` (`self.RoverLog`) (`self.logIndex`))))
  ;[1 1 1] Replay User Inputs
  (if (`self.inputActive`)
    _
    (elif (< (`self.logIndex`) (`KismetArrayLibrary.Array_Length` (`self.RoverLog`)))
      (set `/Game/Simulator/Rover/Blueprint/AIBuggyVH.steering` _item_leftstickx (`self.rover`))
      (set `/Game/Simulator/Rover/Blueprint/AIBuggyVH.thrust` _item_leftsticky (`self.rover`))
      (set `self.logIndex` (+ (`self.logIndex`) 1))
      (else
        (set `self.inputActive` true)))))

(fn `UserConstructionScript`)