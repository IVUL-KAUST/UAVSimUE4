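; Multirotor simulator roll/pitch controller that rotates the craft mesh toward a commanded tilt on one axis, chosen by IsRoll.
; ComputeAngle negates the input, falling back to TrackVar when it is zero, and scales it by MaxAngle.
; The difference from current world angle is clamped to Rate and added as local rotation.
; A velocity-based PID branch is disconnected, so expo and gains have no effect and PID data passes through unchanged.
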(fn `computeAngle`
  (params (_rollpitchValue :type "Float (double-precision)") (_trackVar :type "Float (double-precision)") (_widgetVar :type "Float (double-precision)") (_expo :type "Float (double-precision)") (_rate :type "Float (double-precision)") (_kp :type "Float (double-precision)") (_ki :type "Float (double-precision)") (_kd :type "Float (double-precision)") (_mesh :type "StaticMeshComponent Object Reference") (_pid :type "PidData Structure") (_isRoll :type Boolean) (_lastPos :type "Vector Structure"))
  (returns (_pidData :type "PidData Structure") (lastPosOut :type "Vector Structure"))
  (locals (rollValue :type "Float (double-precision)") (trackXvar :type "Float (double-precision)") (widgetXvar :type "Float (double-precision)") (expoRoll :type "Float (double-precision)") (`Plane mesh` :type "StaticMeshComponent Object Reference") (ErrorX :type "Float (double-precision)") (pidVarXOld :type " Structure") (rollRate :type "Float (double-precision)") (kp :type "Float (double-precision)") (ki :type "Float (double-precision)") (kd :type "Float (double-precision)") (isRoll :type Boolean) (maxAngle :type "Float (double-precision)" :default 30.0) (lastPos :type "Vector Structure") (pidVarX :type "PidData Structure"))
  (bind _rollrate (`local.rollRate`))
  (bind _returnvalue (`KismetMathLibrary.SelectFloat` -1.0 -1.0 (`local.isRoll`)))
  (bind _returnvalue_2 (* (`local.rollValue`) _returnvalue))
  (bind _returnvalue_3 (`KismetMathLibrary.SelectFloat` (* (`local.trackXvar`) _returnvalue) _returnvalue_2 (== _returnvalue_2 0.0)))
  (bind _returnvalue_4 (== 0.0 _returnvalue_3))
  (set `local.rollValue` _rollpitchValue)
  (set `local.trackXvar` _trackVar)
  (set `local.widgetXvar` _widgetVar)
  (set `local.expoRoll` _expo)
  (set `local.rollRate` _rate)
  (set `local.kp` _kp)
  (set `local.ki` _ki)
  (set `local.kd` _kd)
  (set `local.Plane mesh` _mesh)
  (set `local.pidVarX` _pid)
  (set `local.isRoll` _isRoll)
  (if _returnvalue_4
    _
    (else
      _))
  (bind _result (`/Game/Simulator/Multirotor/Blueprints/Constrain.Constrain` (- (* (`KismetMathLibrary.SelectFloat` 0.0 _returnvalue_3 _returnvalue_4) (`local.maxAngle`)) (`KismetMathLibrary.SelectFloat` (.roll (`SceneComponent.K2_GetComponentRotation` (`local.Plane mesh`))) (.pitch (`SceneComponent.K2_GetComponentRotation` (`local.Plane mesh`))) (`local.isRoll`))) (* _rollrate -1.0) _rollrate))
  (if (`local.isRoll`)
    (`SceneComponent.K2_AddLocalRotation` (`local.Plane mesh`) (`KismetMathLibrary.MakeRotator` _result) false false)
    (else
      (`SceneComponent.K2_AddLocalRotation` (`local.Plane mesh`) (`KismetMathLibrary.MakeRotator` 0.0 _result) false false)))
  (set `local.lastPos` (`SceneComponent.K2_GetComponentLocation` (`local.Plane mesh`)))
  (return (`local.pidVarX`) (`local.lastPos`)))