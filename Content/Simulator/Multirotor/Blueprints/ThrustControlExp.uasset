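; Experimental multirotor altitude-hold function that turns axis input into an altitude setpoint and computes thrust, running only while CheckArm is false.
; It cascades deadbanded altitude error into a clamped velocity target, then runs a PID on velocity along the mesh's up vector.
; The clamped output increments thrust, which is added directly to physics velocity along that vector rather than applied as force.
; Thrust zeroes after sustained minimum output.
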(fn `calcThrust`
  (params (_CurAxis :type "Float (double-precision)") (_altMutliplier :type "Float (double-precision)") (_SetPointAlt :type "Float (double-precision)") (_altKp :type "Float (double-precision)") (_altKi :type "Float (double-precision)") (_altKd :type "Float (double-precision)") (_currentThrust :type "Float (double-precision)") (_pidThrust :type "PidData Structure") (_planeMesh :type "StaticMeshComponent Object Reference") (_timeNoThrust :type "Float (double-precision)") (_checkArm :type Boolean))
  (returns (pidOut :type "PidData Structure") (setPointAltOut :type "Float (double-precision)") (currentThrustOut :type "Float (double-precision)") (armOut :type Boolean) (timeNoThrustOut :type "Float (double-precision)"))
  (locals (checkArm :type Boolean :default true) (curAxis :type "Float (double-precision)") (altMultiplier :type "Float (double-precision)" :default 0.0) (SetPointAlt :type "Float (double-precision)") (errorAlt :type "Float (double-precision)") (altKp :type "Float (double-precision)") (altKi :type "Float (double-precision)") (altKd :type "Float (double-precision)") (pidThrustOld :type " Structure") (currentThrust :type "Float (double-precision)") (`Plane mesh` :type "StaticMeshComponent Object Reference") (pidAlitude :type " Structure") (altKp_0 :type "Float (double-precision)" :default 10.0) (timeNoThrust :type "Float (double-precision)") (pidThrust :type "PidData Structure"))
  (bind _setpointalt (`local.SetPointAlt`))
  (bind _z (.z (`SceneComponent.K2_GetComponentLocation` (`local.Plane mesh`))))
  (`|ExecutionSequence`
    (:`then_0`
      (set `local.curAxis` _CurAxis))
    (:`then_1`
      (set `local.altMultiplier` _altMutliplier))
    (:`then_2`
      (set `local.SetPointAlt` _SetPointAlt))
    (:`then_3`
      (set `local.altKp` _altKp))
    (:`then_4`
      (set `local.altKi` _altKi))
    (:`then_5`
      (set `local.altKd` _altKd))
    (:`then_6`
      (set `local.pidThrust` _pidThrust))
    (:`then_7`
      (set `local.currentThrust` _currentThrust))
    (:`then_8`
      (set `local.Plane mesh` _planeMesh))
    (:`then_9`
      (set `local.timeNoThrust` _timeNoThrust))
    (:`then_10`
      (set `local.checkArm` _checkArm))
    (:`then_11`
      ;[1 1 1] Thrust Control
      (if (not (`local.checkArm`))
        (set `local.SetPointAlt` (+ (`local.SetPointAlt`) (* (`local.curAxis`) (`local.altMultiplier`))))
        (bind _output_get (set `local.errorAlt` (- _setpointalt _z)))
        (bind _result (`/Game/Simulator/Multirotor/Blueprints/Constrain.Constrain` _output_get -500.0 500.0))
        (bind _result_2 (`/Game/Simulator/Multirotor/Blueprints/ApplyDeadband.ApplyDeadband` _result 0.1))
        (bind _returnvalue (* _result_2 (`local.altKp_0`)))
        (bind _result_3 (`/Game/Simulator/Multirotor/Blueprints/Constrain.Constrain` _returnvalue -1000.0 1000.0))
        (bind _returnvalue_2 (`PrimitiveComponent.GetPhysicsLinearVelocity` (`local.Plane mesh`) "None"))
        (`KismetSystemLibrary.PrintString` null (`KismetStringLibrary.Concat_StrStr` "Error:" (`KismetStringLibrary.Conv_DoubleToString` _returnvalue)) false false (struct :`G` 0.66 :`B` 1.0 :`A` 1.0) 0.0)
        (bind _returnvalue_3 (`KismetMathLibrary.Dot_VectorVector` (`KismetMathLibrary.GetUpVector` (`SceneComponent.K2_GetComponentRotation` (`local.Plane mesh`))) _returnvalue_2))
        (bind _returnvalue_4 (- _result_3 _returnvalue_3))
        (`KismetSystemLibrary.PrintString` null (`KismetStringLibrary.Concat_StrStr` "Alt:" (`KismetStringLibrary.Conv_DoubleToString` _setpointalt) " C:" (`KismetStringLibrary.Conv_DoubleToString` _z) " " (`KismetStringLibrary.Concat_StrStr` "Velocity: " (`KismetStringLibrary.Conv_DoubleToString` _returnvalue_3)) " V-Error: " (`KismetStringLibrary.Conv_DoubleToString` _returnvalue_4)) false false (struct :`R` 0.138749 :`G` 1.0 :`B` 0.169644 :`A` 1.0) 0.0)
        (bind _returnvalue_5 (`SimulatorFunctions.pidLoop` _returnvalue_4 (`KismetSystemLibrary.GetGameTimeInSeconds` null) (`local.altKp`) (`local.altKi`) (`local.altKd`) (`local.pidThrust`)))
        (bind _output_get_2 (set `local.pidThrust` _returnvalue_5))
        (bind _result_4 (`/Game/Simulator/Multirotor/Blueprints/Constrain.Constrain` (`.output` (break `PidData` _output_get_2)) -15.0 15.0))
        (`KismetSystemLibrary.PrintString` null (`KismetStringLibrary.Concat_StrStr` "PID: " (`KismetStringLibrary.Conv_DoubleToString` _result_4)) false false (struct :`G` 0.66 :`B` 1.0 :`A` 1.0) 0.0)
        (bind _result_5 (`/Game/Simulator/Multirotor/Blueprints/Constrain.Constrain` (+ (`local.currentThrust`) _result_4) 10.0 100.0))
        (bind _output_get_3 (set `local.currentThrust` _result_5))
        (if (== (`local.currentThrust`) 10.0)
          (bind _output_get_4 (set `local.timeNoThrust` (+ 1.0 (`local.timeNoThrust`))))
          (if (> _output_get_4 100.0)
            (set `local.checkArm` false)
            (set `local.currentThrust` 0.0))
          (else
            (set `local.timeNoThrust` 0.0)))
        (`PrimitiveComponent.SetPhysicsLinearVelocity` (`local.Plane mesh`) (* (`KismetMathLibrary.GetUpVector` (`SceneComponent.K2_GetComponentRotation` (`local.Plane mesh`))) _output_get_3) true "None")
        (`KismetSystemLibrary.PrintString` null (`KismetStringLibrary.Concat_StrStr` "Thrust" (`KismetStringLibrary.Conv_DoubleToString` (`local.currentThrust`))) false false (struct :`G` 0.66 :`B` 1.0 :`A` 1.0) 0.0))
      (return (`local.pidThrust`) (`local.SetPointAlt`) (`local.currentThrust`) (`local.checkArm`) (`local.timeNoThrust`)))))