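; Multirotor tracker-following logic that turns X and Y tracker errors into normalized movement outputs.
; When MadeBB is true, ComputeMovement runs a PID loop per axis on game time with shared gains, clamping each output to ±1.
; PID state is passed in and returned so the caller retains it between calls.
; Yaw and altitude setpoint pass through unchanged, as do all values when MadeBB is false.
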(fn `computeMovement`
  (params (_madeBB :type Boolean) (_ErrorX_Tracker :type "Float (double-precision)") (_ErrorY_Tracker :type "Float (double-precision)") (_trackXvar :type "Float (double-precision)") (_trackYvar :type "Float (double-precision)") (_pidTrackVarX :type "PidData Structure") (_pidTrackVarY :type "PidData Structure") (_curYaw :type "Float (double-precision)") (_setPointAlt :type "Float (double-precision)"))
  (returns (_pidTrackVarXOut :type "PidData Structure") (_pidTrackVarYOut :type "PidData Structure") (_trackXvarOut :type "Float (double-precision)") (_trackYvarOut :type "Float (double-precision)") (_curYawOut :type "Float (double-precision)") (_setPointAltOut :type "Float (double-precision)"))
  (locals (madeBB :type Boolean) (ErrorX_Tracker :type "Float (double-precision)") (pidTrackVarXOld :type " Structure") (pidTrackVarYOld :type " Structure") (ErrorY_Tracker :type "Float (double-precision)") (trackXvar :type "Float (double-precision)") (trackYvar :type "Float (double-precision)") (curYaw :type "Float (double-precision)") (setPointAlt :type "Float (double-precision)") (Kp :type "Float (double-precision)" :default 0.006) (Ki :type "Float (double-precision)" :default 0.0) (Kd :type "Float (double-precision)" :default 0.0001) (pidTrackVarX :type "PidData Structure") (pidTrackVarY :type "PidData Structure"))
  (set `local.madeBB` _madeBB)
  (set `local.ErrorX_Tracker` _ErrorX_Tracker)
  (set `local.ErrorY_Tracker` _ErrorY_Tracker)
  (set `local.trackXvar` _trackXvar)
  (set `local.trackYvar` _trackYvar)
  (set `local.pidTrackVarX` _pidTrackVarX)
  (set `local.pidTrackVarY` _pidTrackVarY)
  (set `local.curYaw` _curYaw)
  (set `local.setPointAlt` _setPointAlt)
  ;[1 1 1] PID Loop for Tracker Following
  (if (`local.madeBB`)
    (`|ExecutionSequence`
      (:`then_0`
        (bind _returnvalue (`SimulatorFunctions.pidLoop` (`local.ErrorX_Tracker`) (`KismetSystemLibrary.GetGameTimeInSeconds` null) (`local.Kp`) (`local.Ki`) (`local.Kd`) (`local.pidTrackVarX`)))
        (bind _output_get (set `local.pidTrackVarX` _returnvalue))
        (bind _result (`/Game/Simulator/Multirotor/Blueprints/Constrain.Constrain` (/ (`.output` (break `PidData` _output_get)) 1.0) -1.0 1.0))
        (set `local.trackXvar` _result)
        (`KismetSystemLibrary.PrintString` null (`KismetStringLibrary.Concat_StrStr` "X-Output:" (`KismetStringLibrary.Conv_DoubleToString` _result)) false false (struct :`R` 0.573312 :`B` 1.0 :`A` 1.0) 0.0))
      (:`then_1`
        (bind _returnvalue_2 (`SimulatorFunctions.pidLoop` (`local.ErrorY_Tracker`) (`KismetSystemLibrary.GetGameTimeInSeconds` null) (`local.Kp`) (`local.Ki`) (`local.Kd`) (`local.pidTrackVarY`)))
        (bind _output_get_2 (set `local.pidTrackVarY` _returnvalue_2))
        (bind _result_2 (`/Game/Simulator/Multirotor/Blueprints/Constrain.Constrain` (/ (`.output` (break `PidData` _output_get_2)) 1.0) -1.0 1.0))
        (set `local.trackYvar` _result_2)
        (`KismetSystemLibrary.PrintString` null (`KismetStringLibrary.Concat_StrStr` "Y-Output:" (`KismetStringLibrary.Conv_DoubleToString` _result_2)) false false (struct :`R` 0.573312 :`B` 1.0 :`A` 1.0) 0.0))
      (:`then_2`
        (return (`local.pidTrackVarX`) (`local.pidTrackVarY`) (`local.trackXvar`) (`local.trackYvar`) (`local.curYaw`) (`local.setPointAlt`))))
    (else
      (return (`local.pidTrackVarX`) (`local.pidTrackVarY`) (`local.trackXvar`) (`local.trackYvar`) (`local.curYaw`) (`local.setPointAlt`)))))