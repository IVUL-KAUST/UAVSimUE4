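; YawControl holds a ComputeYaw function that steers the yaw of a mesh in the multirotor simulator.
; It adds yaw rate times yaw input to the passed-in yaw, without delta-time scaling, and returns the result.
; A yaw of exactly zero acts as an uninitialized flag and is replaced by the mesh's world yaw.
; The mesh's world rotation is then set with that yaw, keeping roll and pitch.
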(fn `computeYaw`
  (params (_yawRate :type "Float (double-precision)") (_yawValue :type "Float (double-precision)") (_curYaw :type "Float (double-precision)") (_mesh :type "StaticMeshComponent Object Reference"))
  (returns (_curYawOut :type "Float (double-precision)"))
  (locals (yawRate :type "Float (double-precision)") (yawValue :type "Float (double-precision)") (curYaw :type "Float (double-precision)") (`Plane mesh` :type "StaticMeshComponent Object Reference"))
  (bind _yaw (.yaw (`SceneComponent.K2_GetComponentRotation` (`local.Plane mesh`))))
  (set `local.yawRate` _yawRate)
  (set `local.yawValue` _yawValue)
  (set `local.curYaw` _curYaw)
  (set `local.Plane mesh` _mesh)
  ;[1 1 1] Yaw Control
  (if (== (`local.curYaw`) 0.0)
    (set `local.curYaw` _yaw)
    (else
      (set `local.curYaw` (+ (`local.curYaw`) (* (`local.yawRate`) (`local.yawValue`))))))
  (`SceneComponent.K2_SetWorldRotation` (`local.Plane mesh`) (`KismetMathLibrary.MakeRotator` (.roll (`SceneComponent.K2_GetComponentRotation` (`local.Plane mesh`))) (.pitch (`SceneComponent.K2_GetComponentRotation` (`local.Plane mesh`))) (`local.curYaw`)) false false)
  (`KismetSystemLibrary.PrintString` null (`KismetStringLibrary.Conv_DoubleToString` _yaw) false false (struct :`G` 0.66 :`B` 1.0 :`A` 1.0) 0.0)
  (return (`local.curYaw`)))