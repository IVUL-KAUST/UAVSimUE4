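; Blueprint function for the multirotor simulator that turns a bounding box into X and Y tracking errors relative to screen center.
; It stores the box and screen size, then subtracts the box center from half the screen dimensions.
; The error variables update only when the box's xMax and yMax are positive, and are returned either way.
; Despite its name, it does no UDP or file reading itself.
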(fn `getUdpBoundingBox`
  (params (BoundingBox :type "BoundingBox Structure") (_ScreenWidth :type Integer) (_ScreenHeight :type Integer))
  (returns (ErrorXOut :type "Float (double-precision)") (ErrorYOut :type "Float (double-precision)"))
  (locals (bbExists :type Boolean) (screenWidth :type Integer) (screenHeight :type Integer) (ErrorX_Tracker :type "Float (double-precision)") (ErrorY_Tracker :type "Float (double-precision)") (CurrentBB2 :type Boolean) (CurrentBB :type "BoundingBox Structure"))
  ;[1 1 1] Get BB Text File
  (set `local.screenWidth` _ScreenWidth)
  (set `local.screenHeight` _ScreenHeight)
  (bind _output_get (set `local.CurrentBB` BoundingBox))
  (if (and (> (`.xMax` (break `BoundingBox` _output_get)) 0) (> (`.yMax` (break `BoundingBox` _output_get)) 0))
    (bind (_x _y) (`KismetMathLibrary.BreakVector2D` (break `BoundingBox` _output_get)))
    (set `local.ErrorX_Tracker` (- (/ (`KismetMathLibrary.Conv_IntToDouble` (`local.screenWidth`)) 2.0) _x))
    (set `local.ErrorY_Tracker` (- (/ (`KismetMathLibrary.Conv_IntToDouble` (`local.screenHeight`)) 2.0) _y)))
  (return (`local.ErrorX_Tracker`) (`local.ErrorY_Tracker`)))