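; Position hold function for the simulated multirotor, producing track X/Y corrections when roll, pitch, track and thrust inputs are all zero.
; It latches the mesh's XY location and AltPos as the setpoint, clearing the latch flag on any input.
; Cascaded control along right and forward axes turns proportional position error into clamped velocity targets for PID loops, with UsePos off targeting zero velocity.
; Setpoint and PID state pass through parameters and returns.
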(fn `PositionHold`
  (params (_rollValue :type "Float (double-precision)") (_pitchValue :type "Float (double-precision)") (_trackY :type "Float (double-precision)") (_trackX :type "Float (double-precision)") (_setPoint :type Boolean) (_curPos :type "Vector Structure") (_pidXpos :type "PidData Structure") (_pidYpos :type "PidData Structure") (_planeMesh :type "StaticMeshComponent Object Reference") (_thrustValue :type "Float (double-precision)") (_altPos :type "Float (double-precision)") (_usePos :type Boolean))
  (returns (trackXOut :type "Float (double-precision)") (trackYOut :type "Float (double-precision)") (pidXOut :type "PidData Structure") (pidYOut :type "PidData Structure") (setPointOut :type Boolean) (curPosOut :type "Vector Structure"))
  (locals (rollValue :type "Float (double-precision)") (trackXvar :type "Float (double-precision)") (trackYvar :type "Float (double-precision)") (pitchValue :type "Float (double-precision)") (setSetPoint :type Boolean) (currentPos :type "Vector Structure") (Kp :type "Float (double-precision)" :default 0.01) (Ki :type "Float (double-precision)") (Kd :type "Float (double-precision)" :default 0.0) (`Plane mesh` :type "StaticMeshComponent Object Reference") (thrustValue :type "Float (double-precision)") (deadband :type "Float (double-precision)" :default 1.0) (altPos :type "Float (double-precision)") (kPpos :type "Float (double-precision)" :default 2.0) (usePos :type Boolean) (pidXfix :type "PidData Structure") (pidYfix :type "PidData Structure"))
  (bind _plane_mesh (`local.Plane mesh`))
  (bind _returnvalue (`SceneComponent.K2_GetComponentRotation` _plane_mesh))
  (bind _returnvalue_2 (- (`local.currentPos`) (`SceneComponent.K2_GetComponentLocation` _plane_mesh)))
  (set `local.rollValue` _rollValue)
  (set `local.pitchValue` _pitchValue)
  (set `local.trackYvar` _trackY)
  (set `local.trackXvar` _trackX)
  (set `local.setSetPoint` _setPoint)
  (set `local.currentPos` _curPos)
  (set `local.pidXfix` _pidXpos)
  (set `local.pidYfix` _pidYpos)
  (set `local.Plane mesh` _planeMesh)
  (set `local.thrustValue` _thrustValue)
  (set `local.altPos` _altPos)
  (set `local.usePos` _usePos)
  (if (and (== 0.0 (`local.rollValue`)) (== 0.0 (`local.trackXvar`)) (== 0.0 (`local.trackYvar`)) (== 0.0 (`local.pitchValue`)) (== 0.0 (`local.thrustValue`)))
    (if (`local.setSetPoint`)
      (`KismetSystemLibrary.PrintString` null (`KismetStringLibrary.Conv_VectorToString` _returnvalue_2) false false (struct :`R` 0.683879 :`G` 1.0 :`B` 0.0478 :`A` 1.0) 0.0)
      (`|ExecutionSequence`
        (:`then_0`
          (bind _result (`/Game/Simulator/Multirotor/Blueprints/ApplyDeadband.ApplyDeadband` (`KismetMathLibrary.Dot_VectorVector` (`KismetMathLibrary.GetRightVector` _returnvalue) _returnvalue_2) (`local.deadband`)))
          (bind _returnvalue_3 (* (* _result (`local.kPpos`)) (`KismetMathLibrary.SelectFloat` 1.0 0.0 (`local.usePos`))))
          (bind _result_2 (`/Game/Simulator/Multirotor/Blueprints/Constrain.Constrain` _returnvalue_3 -500.0 500.0))
          (bind _returnvalue_4 (`PrimitiveComponent.GetPhysicsLinearVelocity` (`local.Plane mesh`) "None"))
          (bind _returnvalue_5 (`KismetMathLibrary.Dot_VectorVector` (`KismetMathLibrary.GetRightVector` (`SceneComponent.K2_GetComponentRotation` (`local.Plane mesh`))) _returnvalue_4))
          (bind _returnvalue_6 (- _result_2 _returnvalue_5))
          (`KismetSystemLibrary.PrintString` null (`KismetStringLibrary.Concat_StrStr` (`KismetStringLibrary.Conv_DoubleToString` _returnvalue_3) " vel:" (`KismetStringLibrary.Conv_DoubleToString` _returnvalue_5) " dist: " "" " err:" (`KismetStringLibrary.Conv_DoubleToString` _returnvalue_6)) false false (struct :`G` 1.0 :`B` 0.045079 :`A` 1.0) 0.0)
          (bind _returnvalue_7 (`SimulatorFunctions.pidLoop` _returnvalue_6 (`KismetSystemLibrary.GetGameTimeInSeconds` null) (`local.Kp`) (`local.Ki`) (`local.Kd`) (`local.pidXfix`)))
          (bind _output_get (set `local.pidXfix` _returnvalue_7))
          (`KismetSystemLibrary.PrintString` null (`KismetStringLibrary.Conv_DoubleToString` (`.output` (break `PidData` _output_get))) false false (struct :`R` 0.683879 :`G` 1.0 :`B` 0.0478 :`A` 1.0) 0.0)
          (bind _result_3 (`/Game/Simulator/Multirotor/Blueprints/Constrain.Constrain` (* (`.output` (break `PidData` _output_get)) -1.0) -0.5 0.5))
          (bind _result_4 (`/Game/Simulator/Multirotor/Blueprints/ApplyDeadband.ApplyDeadband` _result_3 0.01))
          (set `local.trackXvar` _result_4))
        (:`then_1`
          (bind _result_5 (`/Game/Simulator/Multirotor/Blueprints/ApplyDeadband.ApplyDeadband` (`KismetMathLibrary.Dot_VectorVector` (`KismetMathLibrary.GetForwardVector` _returnvalue) _returnvalue_2) (`local.deadband`)))
          (bind _result_6 (`/Game/Simulator/Multirotor/Blueprints/Constrain.Constrain` (* (* _result_5 (`local.kPpos`)) (`KismetMathLibrary.SelectFloat` 1.0 0.0 (`local.usePos`))) -500.0 500.0))
          (bind _returnvalue_8 (`PrimitiveComponent.GetPhysicsLinearVelocity` (`local.Plane mesh`) "None"))
          (bind _returnvalue_9 (`SimulatorFunctions.pidLoop` (- _result_6 (`KismetMathLibrary.Dot_VectorVector` (`KismetMathLibrary.GetForwardVector` (`SceneComponent.K2_GetComponentRotation` (`local.Plane mesh`))) _returnvalue_8)) (`KismetSystemLibrary.GetGameTimeInSeconds` null) (`local.Kp`) (`local.Ki`) (`local.Kd`) (`local.pidYfix`)))
          (bind _output_get_2 (set `local.pidYfix` _returnvalue_9))
          (bind _result_7 (`/Game/Simulator/Multirotor/Blueprints/Constrain.Constrain` (`.output` (break `PidData` _output_get_2)) -0.5 0.5))
          (bind _result_8 (`/Game/Simulator/Multirotor/Blueprints/ApplyDeadband.ApplyDeadband` _result_7 0.01))
          (set `local.trackYvar` _result_8))
        (:`then_2`
          (return (`local.trackXvar`) (`local.trackYvar`) (`local.pidXfix`) (`local.pidYfix`) (`local.setSetPoint`) (`local.currentPos`))))
      (else
        (bind _output_get_3 (set `local.currentPos` (`KismetMathLibrary.MakeVector` (.x (`SceneComponent.K2_GetComponentLocation` (`local.Plane mesh`))) (.y (`SceneComponent.K2_GetComponentLocation` (`local.Plane mesh`))) (`local.altPos`))))
        (set `local.setSetPoint` true)
        (`KismetSystemLibrary.PrintString` null (`KismetStringLibrary.Conv_VectorToString` _output_get_3) false false (struct :`R` 0.683879 :`G` 1.0 :`B` 0.0478 :`A` 1.0) 0.0)
        (return (`local.trackXvar`) (`local.trackYvar`) (`local.pidXfix`) (`local.pidYfix`) (`local.setSetPoint`) (`local.currentPos`))))
    (else
      (set `local.setSetPoint` false)
      (return (`local.trackXvar`) (`local.trackYvar`) (`local.pidXfix`) (`local.pidYfix`) (`local.setSetPoint`) (`local.currentPos`)))))