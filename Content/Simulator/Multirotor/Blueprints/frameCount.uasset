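; Frame-count Blueprint in the multirotor simulator that turns a frame number into a zero-padded string for frame file naming.
; GetFrameString picks a zero prefix through nested SelectString threshold checks and prepends it to the number.
; The result is six digits wide below 100000; larger counts still get one leading zero, so the width grows.
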(fn `getFrameString`
  (params (_CountFrames :type Integer))
  (returns (_FrameString :type String))
  (locals (countFrames :type Integer))
  (bind _countframes (`local.countFrames`))
  (set `local.countFrames` _CountFrames)
  (return (`KismetStringLibrary.Concat_StrStr` (`KismetMathLibrary.SelectString` "00000" (`KismetMathLibrary.SelectString` "0000" (`KismetMathLibrary.SelectString` "000" (`KismetMathLibrary.SelectString` "00" "0" (< _countframes 10000)) (< _countframes 1000)) (< _countframes 100)) (< _countframes 10)) (`KismetStringLibrary.Conv_IntToString` _countframes))))