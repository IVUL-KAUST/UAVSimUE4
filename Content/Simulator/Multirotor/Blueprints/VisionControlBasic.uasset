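; Vision control for the simulated multirotor, turning a target bounding box into X/Y tracking errors on the Multirotor.
; Input toggles switch tracking with CamLogger UDP logging, and pick ground truth or external tracker as error source.
; While tracking, Tick computes ground-truth boxes from a scene capture, passing them to CamLogger and SendBBTextfile on localhost.
; In vision mode, SimUDPReceiver's box supplies the errors, even with tracking off; the file-based reader is hard-disabled.
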(event `InputAction|StartTracking`
  (params (Key :type "Key Structure" :default "AnyKey"))
  (bind _multirotor (`self.multirotor`))
  (:`Pressed`
    (`/Engine/EditorBlueprintResources/StandardMacros.FlipFlop`
      (:`A`
        (set `self.trackingStart` true)
        (set `/Game/Simulator/Multirotor/Blueprints/MultiRotorMbzirc.trackingStart` true _multirotor)
        (if true
          (bind _outactors (`GameplayStatics.GetAllActorsOfClass` "/Game/Simulator/Camera/CamLogger.CamLogger_C"))
          (set `/Game/Simulator/Camera/CamLogger.EnableLogUDP` true (`KismetArrayLibrary.Array_Get` _outactors))))
      (:`B`
        (set `self.trackingStart` false)
        (set `/Game/Simulator/Multirotor/Blueprints/MultiRotorMbzirc.trackingStart` false _multirotor)
        (if true
          (bind _outactors_2 (`GameplayStatics.GetAllActorsOfClass` "/Game/Simulator/Camera/CamLogger.CamLogger_C"))
          (set `/Game/Simulator/Camera/CamLogger.EnableLogUDP` false (`KismetArrayLibrary.Array_Get` _outactors_2)))))))

(event `InputAction|toggleBoundingBox`
  (params (Key :type "Key Structure" :default "AnyKey"))
  (:`Pressed`
    (`/Engine/EditorBlueprintResources/StandardMacros.FlipFlop`
      (:`A`
        (set `self.useGtBB` false)
        (if (`self.trackingStart`)
          (set `self.trackingStart` true)))
      (:`B`
        (set `self.useGtBB` true)))))

(event `self.ReceiveTick`
  (params (DeltaSeconds :type "Float (single-precision)"))
  (bind _multirotor (`self.multirotor`))
  (bind _multirotor_2 (`self.multirotor`))
  (bind _multirotor_3 (`self.multirotor`))
  (if true
    (`|ExecutionSequence`
      (:`then_1`
        ;[1 1 1] Use GT to move Copter
        (if (`self.trackingStart`)
          (bind (__errorxtrackerout __errorytrackerout _curbbout) (`/Game/Simulator/Multirotor/Blueprints/GTcomppute.calcMovementFromGT` (`/Game/Simulator/Multirotor/Blueprints/MultiRotorMbzirc.SceneCaptureComponent2D1` (`self.multirotor`)) 640 360))
          (`|ExecutionSequence`
            (:`then_0`
              (bind _output_get (set `/Game/Simulator/Multirotor/Blueprints/MultiRotorMbzirc.CurrentBB` _curbbout _multirotor))
              (bind _outactors (`GameplayStatics.GetAllActorsOfClass` "/Game/Simulator/Camera/CamLogger.CamLogger_C"))
              (bind _output_get_2 (set `/Game/Simulator/Camera/CamLogger.CurrentBB` _output_get (`KismetArrayLibrary.Array_Get` _outactors)))
              (`SimulatorFunctions.sendBBTextfile` "127.0.0.1" 25001 "0" _output_get_2)
              (`KismetSystemLibrary.PrintString` (`KismetStringLibrary.Concat_StrStr` (`KismetStringLibrary.Conv_Vector2dToString` (`.center` (break `BoundingBox` _output_get_2))) "  " "GT") true false (struct :`G` 0.66 :`B` 1.0 :`A` 1.0) 0.0))
            (:`then_1`
              (if (`self.useGtBB`)
                (bind _output_get_3 (set `/Game/Simulator/Multirotor/Blueprints/MultiRotorMbzirc.ErrorX_Tracker` __errorxtrackerout _multirotor))
                (set `/Game/Simulator/Multirotor/Blueprints/MultiRotorMbzirc.ErrorY_Tracker` __errorytrackerout _multirotor)
                (`KismetSystemLibrary.PrintString` (`KismetStringLibrary.Conv_DoubleToString` _output_get_3) true false (struct :`G` 0.66 :`B` 1.0 :`A` 1.0) 0.0))))))
      (:`then_2`
        ;[1 1 1] Get Bbox From Tracker
        (if (not (`self.useGtBB`))
          (`|ExecutionSequence`
            (:`then_0`
              (if true
                (bind _outactors_2 (`GameplayStatics.GetAllActorsOfClass` "/Game/Simulator/DefaultLevel/SimUDPReceiver.SimUDPReceiver_C"))
                (bind (_errorxout _erroryout) (`/Game/Simulator/Multirotor/Blueprints/GetUdpBoundingBox.getUdpBoundingBox` (`/Game/Simulator/DefaultLevel/SimUDPReceiver.recvBB` (`KismetArrayLibrary.Array_Get` _outactors_2)) 640 360))
                (bind _output_get_4 (set `/Game/Simulator/Multirotor/Blueprints/MultiRotorMbzirc.ErrorX_Tracker` _errorxout _multirotor_2))
                (set `/Game/Simulator/Multirotor/Blueprints/MultiRotorMbzirc.ErrorY_Tracker` _erroryout _multirotor_2)
                (`KismetSystemLibrary.PrintString` (`KismetStringLibrary.Concat_StrStr` (`KismetStringLibrary.Conv_DoubleToString` _output_get_4) " " "Vision") false false (struct :`G` 0.66 :`B` 1.0 :`A` 1.0) 0.0)
                (else
                  (bind (_errorxout_2 _erroryout_2) (`/Game/Simulator/Multirotor/Blueprints/GetBoundingBox.getBoundingBox` "R:/frames/img/" 640 360))
                  (set `/Game/Simulator/Multirotor/Blueprints/MultiRotorMbzirc.ErrorX_Tracker` _errorxout_2 _multirotor_3)
                  (set `/Game/Simulator/Multirotor/Blueprints/MultiRotorMbzirc.ErrorY_Tracker` _erroryout_2 _multirotor_3))))
            (:`then_1`
              (`/Engine/EditorBlueprintResources/StandardMacros.DoOnce` false
                (:`Completed`
                  (`KismetSystemLibrary.PrintString` "Vision Enabled" true false (struct :`G` 0.66 :`B` 1.0 :`A` 1.0) 5.0))))))))))

(fn `UserConstructionScript`)