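; GoToWaypoint is a multirotor simulator function that supplies altitude setpoint and target position for flying to a desired waypoint.
; It passes the target Z through as altitude, with zero yaw and the setpoint flag always on.
; A deadbanded distance from the plane mesh, printed for debugging, drives ReachedOut, which is true while the waypoint is not reached.
; An unconnected branch holds unused rate-limited vertical axis logic.
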(fn `GoToWaypoint`
  (params (_desiredPos :type "Vector Structure") (_planeMesh :type "StaticMeshComponent Object Reference"))
  (returns (zOut :type "Float (double-precision)") (yawOut :type "Float (double-precision)") (reachedOut :type Boolean) (setPointOut :type Boolean) (goToPos :type "Vector Structure"))
  (locals (currentPos :type "Vector Structure") (trackXvar :type "Float (double-precision)") (trackYvar :type "Float (double-precision)") (curAxis :type "Float (double-precision)") (desiredPos :type "Vector Structure") (PlaneMesh :type "StaticMeshComponent Object Reference") (posNotReached :type Boolean) (maxRate :type "Float (double-precision)" :default 500.0) (SetPointAlt :type "Float (double-precision)") (setSetPoint :type Boolean))
  (bind _output_get (set `local.desiredPos` _desiredPos))
  (bind _output_get_2 (set `local.PlaneMesh` _planeMesh))
  (set `local.SetPointAlt` (.z _output_get))
  (set `local.setSetPoint` true)
  (bind _result (`/Game/Simulator/Multirotor/Blueprints/ApplyDeadband.ApplyDeadband` (`KismetMathLibrary.VSize` (- _output_get (`SceneComponent.K2_GetComponentLocation` _output_get_2))) 1.0))
  (set `local.posNotReached` (!= _result 0.0))
  (`KismetSystemLibrary.PrintString` null (`KismetStringLibrary.Conv_DoubleToString` _result) true false (struct :`G` 0.66 :`B` 1.0 :`A` 1.0) 0.0)
  (return (`local.SetPointAlt`) 0.0 (`local.posNotReached`) (`local.setSetPoint`) (`local.desiredPos`)))