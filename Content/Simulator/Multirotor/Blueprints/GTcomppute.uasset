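; Multirotor simulator Blueprint that computes tracking error from a ground-truth (GT) bounding box instead of a tracker estimate.
; CalcMovementFromGT gets the box from a SceneCapture component and subtracts its center from the screen center on X and Y.
; It returns both pixel errors and the box.
; The errors are returned unclamped, as the Constrain results are not used.
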(fn `calcMovementFromGT`
  (params (_sceneCapture :type "SceneCaptureComponent2D Object Reference") (_screenWidth :type Integer) (_screenHeight :type Integer))
  (returns (_errorXTrackerOut :type "Float (double-precision)") (_errorYTrackerOut :type "Float (double-precision)") (curBBOut :type "BoundingBox Structure"))
  (locals (SceneCaptureComponent2D :type "SceneCaptureComponent2D Object Reference") (screenWidth :type Integer) (screenHeight :type Integer) (ErrorX_Tracker :type "Float (double-precision)") (ErrorY_Tracker :type "Float (double-precision)") (CurrentBB :type "BoundingBox Structure"))
  ;[1 1 1] Use GT BoundingBox
  (bind _returnvalue (`SimulatorFunctions.CaptureComponent2D_BBImage` _sceneCapture))
  (bind _output_get (set `local.CurrentBB` _returnvalue))
  (bind (_x _y) (`KismetMathLibrary.BreakVector2D` (break `BoundingBox` _output_get)))
  (bind _returnvalue_2 (- (/ (`KismetMathLibrary.Conv_IntToDouble` _screenWidth) 2.0) _x))
  (`/Game/Simulator/Multirotor/Blueprints/Constrain.Constrain` _returnvalue_2 -50.0 50.0)
  (bind _returnvalue_3 (- (/ (`KismetMathLibrary.Conv_IntToDouble` _screenHeight) 2.0) _y))
  (`/Game/Simulator/Multirotor/Blueprints/Constrain.Constrain` _returnvalue_3 -50.0 50.0)
  (bind _output_get_2 (set `local.ErrorX_Tracker` _returnvalue_2))
  (set `local.ErrorY_Tracker` _returnvalue_3)
  (`KismetSystemLibrary.PrintString` null (`KismetStringLibrary.Conv_DoubleToString` _output_get_2) false false (struct :`G` 0.66 :`B` 1.0 :`A` 1.0) 0.0)
  (return (`local.ErrorX_Tracker`) (`local.ErrorY_Tracker`) (`local.CurrentBB`)))