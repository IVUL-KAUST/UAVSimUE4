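; LogData provides MakeLog, which records UAV and target tracking data for the multirotor simulator.
; When the toggle is on, it samples world position, rotation and physics velocity from the UAV mesh and the target skeletal mesh.
; Velocities are projected onto each mesh's own forward, right and up axes, giving body-frame values.
; SaveTrackingLog receives these with the frame string, which also names the .log file in the given directory.
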(fn `makeLog`
  (params (_frameString :type String) (_mesh :type "StaticMeshComponent Object Reference") (_skmesh :type "SkeletalMeshComponent Object Reference") (_directory :type String) (toggleLog :type Boolean))
  (locals (`Plane mesh` :type "StaticMeshComponent Object Reference"))
  (bind _returnvalue (`SceneComponent.K2_GetComponentRotation` _skmesh))
  (bind _plane_mesh (`local.Plane mesh`))
  (bind _returnvalue_2 (`SceneComponent.K2_GetComponentRotation` _plane_mesh))
  (if toggleLog
    (set `local.Plane mesh` _mesh)
    ;[1 1 1] UAV Log Data
    (bind _returnvalue_3 (`PrimitiveComponent.GetPhysicsLinearVelocity` _plane_mesh "None"))
    (bind _returnvalue_4 (`PrimitiveComponent.GetPhysicsLinearVelocity` _skmesh "None"))
    ;[1 1 1] Save Log
    (`SimulatorFunctions.saveTrackingLog` (`KismetStringLibrary.Concat_StrStr` _directory "/" _frameString ".log") _frameString (`SceneComponent.K2_GetComponentLocation` _plane_mesh) (`SceneComponent.K2_GetComponentLocation` _skmesh) (`KismetMathLibrary.MakeVector` (.roll _returnvalue_2) (.pitch _returnvalue_2) (.yaw _returnvalue_2)) (`KismetMathLibrary.MakeVector` (.roll _returnvalue) (.pitch _returnvalue) (.yaw _returnvalue)) (`KismetMathLibrary.MakeVector` (`KismetMathLibrary.Dot_VectorVector` _returnvalue_3 (`KismetMathLibrary.GetForwardVector` _returnvalue_2)) (`KismetMathLibrary.Dot_VectorVector` _returnvalue_3 (`KismetMathLibrary.GetRightVector` _returnvalue_2)) (`KismetMathLibrary.Dot_VectorVector` _returnvalue_3 (`KismetMathLibrary.GetUpVector` _returnvalue_2))) (`KismetMathLibrary.MakeVector` (`KismetMathLibrary.Dot_VectorVector` _returnvalue_4 (`KismetMathLibrary.GetForwardVector` _returnvalue)) (`KismetMathLibrary.Dot_VectorVector` _returnvalue_4 (`KismetMathLibrary.GetRightVector` _returnvalue)) (`KismetMathLibrary.Dot_VectorVector` _returnvalue_4 (`KismetMathLibrary.GetUpVector` _returnvalue))))))