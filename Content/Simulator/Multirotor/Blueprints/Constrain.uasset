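; Blueprint function Constrain in the multirotor simulator that clamps a value between a minimum and a maximum.
; It checks the upper bound first, then the lower, returning the breached limit or the unchanged value.
; Each branch feeds a SelectFloat that repeats its comparison, and both lower-bound paths perform the same selection.
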(fn `Constrain`
  (params (value :type "Float (double-precision)") (min :type "Float (double-precision)") (max :type "Float (double-precision)"))
  (returns (result :type "Float (double-precision)"))
  (locals (Output :type "Float (double-precision)"))
  (bind _returnvalue (> value max))
  (bind _returnvalue_2 (< value min))
  (bind _returnvalue_3 (`KismetMathLibrary.SelectFloat` min value _returnvalue_2))
  (if _returnvalue
    (set `local.Output` (`KismetMathLibrary.SelectFloat` max value _returnvalue))
    (elif _returnvalue_2
      (set `local.Output` _returnvalue_3)
      (else
        (set `local.Output` _returnvalue_3))))
  (return (`local.Output`)))