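; MBZIRC simulator quadcopter flown by axis input, with arming, tracker following and waypoint flight.
; BeginPlay attaches cover, gimbal, legs and motors to PlaneMesh sockets.
; Tick feeds tracker, waypoint and position-hold targets into PID thrust and roll/pitch control plus yaw control, spins motors, poses legs and counter-rotates the gimbal to stay level.
; Waypoint loading is unwired; Space saves hard-coded test waypoints to a fixed path.
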(event `self.ReceiveBeginPlay`
  ;[1 1 1] Set Copter Elevation at Beginning
  (`|ExecutionSequence`
    (:`then_0`
      (set `self.SetPointAlt` (.z (`SceneComponent.K2_GetComponentLocation` (`self.PlaneMesh`)))))
    (:`then_1`
      (`|ExecutionSequence`
        (:`then_0`
          ;[1 1 1] Shell/Gimbal
          (bind _returnvalue (`AddComponent|StaticMeshComponent_0` :`bManualAttachment` true)) ; Cover
          (bind _output_get (set `self.Cover` _returnvalue))
          (`SceneComponent.K2_AttachToComponent` _output_get (`self.PlaneMesh`) "shell" "KeepRelative" "KeepRelative" "KeepRelative" true))
        (:`then_1`
          (bind _returnvalue_2 (`AddComponent|StaticMeshComponent_1`)) ; Gimbal Base
          (bind _output_get_2 (set `self.gimbalBase` _returnvalue_2))
          (`SceneComponent.K2_AttachToComponent` _output_get_2 (`self.PlaneMesh`) "gimbalatt" "KeepRelative" "KeepRelative" "KeepRelative" true))
        (:`then_2`
          ;[1 1 1] Legs
          (`|ExecutionSequence`
            (:`then_0`
              (bind _returnvalue_3 (`AddComponent|StaticMeshComponent_2` :`bManualAttachment` true)) ; Leg
              (bind _output_get_3 (set `self.Leg1` _returnvalue_3))
              (`SceneComponent.K2_AttachToComponent` _output_get_3 (`self.gimbalBase`) "Leg1" "KeepRelative" "KeepRelative" "KeepRelative" true))
            (:`then_1`
              (bind _returnvalue_4 (`AddComponent|StaticMeshComponent_4` :`bManualAttachment` true)) ; Leg
              (bind _output_get_4 (set `self.Leg2` _returnvalue_4))
              (`SceneComponent.K2_AttachToComponent` _output_get_4 (`self.gimbalBase`) "Leg2" "KeepRelative" "KeepRelative" "KeepRelative" true))
            (:`then_2`
              (bind _returnvalue_5 (`AddComponent|StaticMeshComponent_5` :`bManualAttachment` true)) ; Leg
              (bind _output_get_5 (set `self.Leg3` _returnvalue_5))
              (`SceneComponent.K2_AttachToComponent` _output_get_5 (`self.gimbalBase`) "Leg3" "KeepRelative" "KeepRelative" "KeepRelative" true))
            (:`then_3`
              (bind _returnvalue_6 (`AddComponent|StaticMeshComponent_6` :`bManualAttachment` true)) ; Leg
              (bind _output_get_6 (set `self.Leg4` _returnvalue_6))
              (`SceneComponent.K2_AttachToComponent` _output_get_6 (`self.gimbalBase`) "Leg4" "KeepRelative" "KeepRelative" "KeepRelative" true))))
        (:`then_3`
          ;[1 1 1] Motors
          (`|ExecutionSequence`
            (:`then_0`
              (bind _returnvalue_7 (`AddComponent|StaticMeshComponent_3` :`bManualAttachment` true)) ; Motor
              (bind _output_get_7 (set `self.Motor1` _returnvalue_7))
              (`SceneComponent.K2_AttachToComponent` _output_get_7 (`self.PlaneMesh`) "motor_1" "KeepRelative" "KeepRelative" "KeepRelative" true))
            (:`then_1`
              (bind _returnvalue_8 (`AddComponent|StaticMeshComponent_7` :`bManualAttachment` true)) ; Motor
              (bind _output_get_8 (set `self.Motor2` _returnvalue_8))
              (`SceneComponent.K2_AttachToComponent` _output_get_8 (`self.PlaneMesh`) "motor_2" "KeepRelative" "KeepRelative" "KeepRelative" true))
            (:`then_2`
              (bind _returnvalue_9 (`AddComponent|StaticMeshComponent_8` :`bManualAttachment` true)) ; Motor
              (bind _output_get_9 (set `self.Motor3` _returnvalue_9))
              (`SceneComponent.K2_AttachToComponent` _output_get_9 (`self.PlaneMesh`) "motor_3" "KeepRelative" "KeepRelative" "KeepRelative" true))
            (:`then_3`
              (bind _returnvalue_10 (`AddComponent|StaticMeshComponent_9` :`bManualAttachment` true)) ; Motor
              (bind _output_get_10 (set `self.Motor4` _returnvalue_10))
              (`SceneComponent.K2_AttachToComponent` _output_get_10 (`self.PlaneMesh`) "motor_4" "KeepRelative" "KeepRelative" "KeepRelative" true))))))))

(event `self.ReceiveTick`
  (params (DeltaSeconds :type "Float (single-precision)"))
  (bind _returnvalue (`KismetMathLibrary.MakeRotator` 0.0 0.0 50.0))
  (bind _returnvalue_2 (`KismetMathLibrary.MakeRotator` 0.0 0.0 50.0))
  (bind _currentwaypoint (`self.currentWayPoint`))
  (bind _legpos (`self.legPos`))
  (bind _returnvalue_3 (`SceneComponent.K2_GetComponentLocation` (`self.PlaneMesh`)))
  (bind _returnvalue_4 (`KismetMathLibrary.MakeRotator` (`self.legPos`) 0.0 0.0))
  (bind _returnvalue_5 (+ (`self.legPos`) 2.0))
  ;[1 1 1] Event Ticks
  (`|ExecutionSequence`
    (:`then_0`
      ;[1 1 1] PID Loop for Tracker Following
      (if (`self.trackingStart`)
        (if true
          (bind (__pidtrackvarxout __pidtrackvaryout __trackxvarout __trackyvarout __curyawout __setpointaltout) (`/Game/Simulator/Multirotor/Blueprints/TrackerFollowing.computeMovement` true (`self.ErrorX_Tracker`) (`self.ErrorY_Tracker`) (`self.trackXvar`) (`self.trackYvar`) (`self.pidTrackXVar`) (`self.pidTrackYVar`) (`self.curYaw`) (`self.SetPointAlt`)))
          (set `self.pidTrackXVar` __pidtrackvarxout)
          (set `self.pidTrackYVar` __pidtrackvaryout)
          (set `self.trackXvar` __trackxvarout)
          (set `self.trackYvar` __trackyvarout)
          (set `self.curYaw` __curyawout)
          (set `self.SetPointAlt` __setpointaltout))))
    (:`then_2`
      (`|ExecutionSequence`
        (:`then_0`
          (if (`self.switchMode`)
            (if (`self.checkArm`)
              ;[1 1 1] Arm and Reset
              (if (`self.ArmCopter`)
                (bind _output_get (set `self.SetPointAlt` (+ (.z _returnvalue_3) 10.0 0.0)))
                (set `self.LastSetPointAlt` _output_get)
                (set `self.currentPos` _returnvalue_3)
                (set `self.checkArm` true)
                (set `self.ArmCopter` false)
                (set `self.timeNoThrust` 0.0)
                (set `self.trackXvar` 0.0)
                (set `self.trackYvar` 0.0)
                (set `self.currentThrust` 0.0)
                (set `self.setSetPoint` false)
                (else
                  ;[1 1 1] Turn On Hover
                  (if (> (`self.curAxis`) 0.5)
                    (set `self.checkArm` false))))
              (else
                (`|ExecutionSequence`
                  (:`then_0`
                    ;[1 1 1] Go To Waypoint Sent
                    (if (`self.waypointsActive`)
                      (set `self.posNotReached` true)
                      (if (< (`self.currentWayPoint`) (`KismetArrayLibrary.Array_Length` (`self.wayPoints`)))
                        (set `self.goToPos` (`KismetArrayLibrary.Array_Get` (`self.wayPoints`) _currentwaypoint))
                        (`KismetSystemLibrary.PrintString` (`KismetStringLibrary.Conv_IntToString` _currentwaypoint) false false (struct :`G` 0.66 :`B` 1.0 :`A` 1.0) 0.0)
                        (if (`self.posNotReached`)
                          (bind (_zout _yawout _reachedout _setpointout _gotopos) (`/Game/Simulator/Multirotor/Blueprints/GoToWaypoint.GoToWaypoint` (`self.goToPos`) (`self.PlaneMesh`)))
                          (set `self.SetPointAlt` _zout)
                          (bind _output_get_2 (set `self.posNotReached` _reachedout))
                          (set `self.setSetPoint` _setpointout)
                          (set `self.currentPos` _gotopos)
                          (if (not _output_get_2)
                            (set `self.currentWayPoint` (+ (`self.currentWayPoint`) 1))
                            (set `self.posNotReached` true)))
                        (else
                          (set `self.currentWayPoint` 0)
                          (set `self.waypointsActive` false)
                          (set `self.posNotReached` false)))))
                  (:`then_1`
                    (`|ExecutionSequence`
                      (:`then_0`
                        ;[1 1 1] Thrust/Elevation Auto
                        (if (not (`self.checkArm`))
                          (bind (_pidout _setpointaltout _currentthrustout _armout _timenothrustout) (`/Game/Simulator/Multirotor/Blueprints/ThrustControlExp.calcThrust` (`self.curAxis`) (`self.altMultiplier`) (`self.SetPointAlt`) (`self.altKp`) (`self.altKi`) (`self.altKd`) (`self.currentThrust`) (`self.pidThrust`) (`self.PlaneMesh`) (`self.timeNoThrust`) (`self.checkArm`)))
                          (set `self.pidThrust` _pidout)
                          (set `self.SetPointAlt` _setpointaltout)
                          (set `self.currentThrust` _currentthrustout)
                          (set `self.checkArm` _armout)
                          (set `self.timeNoThrust` _timenothrustout)))
                      (:`then_1`
                        ;[1 1 1] Yaw Auto
                        (if (not (`self.checkArm`))
                          (bind __curyawout_2 (`/Game/Simulator/Multirotor/Blueprints/YawControl.computeYaw` 2.0 (`self.yawValue`) (`self.curYaw`) (`self.PlaneMesh`)))
                          (set `self.curYaw` __curyawout_2)))
                      (:`then_2`
                        (`|ExecutionSequence`
                          (:`then_0`
                            ;[1 1 1] Position Hold X/Y
                            (if (not (`self.checkArm`))
                              (bind (_trackxout _trackyout _pidxout _pidyout _setpointout_2 _curposout) (`/Game/Simulator/Multirotor/Blueprints/PositionHold.PositionHold` (`self.rollValue`) (`self.pitchValue`) (`self.trackYvar`) (`self.trackXvar`) (`self.setSetPoint`) (`self.currentPos`) (`self.pidPosX`) (`self.pidPosY`) (`self.PlaneMesh`) (`self.curAxis`) (`self.SetPointAlt`) (`self.posNotReached`)))
                              (set `self.trackXvar` _trackxout)
                              (set `self.trackYvar` _trackyout)
                              (set `self.pidPosX` _pidxout)
                              (set `self.pidPosY` _pidyout)
                              (set `self.setSetPoint` _setpointout_2)
                              (set `self.currentPos` _curposout)))
                          (:`then_1`
                            ;[1 1 1] Roll Auto
                            (if (not (`self.checkArm`))
                              (bind __piddata (`/Game/Simulator/Multirotor/Blueprints/RollPitchControlExp.computeAngle` (`self.rollValue`) (`self.trackXvar`) (`self.widgetXvar`) 5000.0 3.0 0.007 0.0 0.003 (`self.PlaneMesh`) (`self.pidXVar`) true))
                              (set `self.pidXVar` __piddata)
                              (set `self.trackXvar` 0.0)))
                          (:`then_2`
                            ;[1 1 1] Pitch Auto
                            (if (not (`self.checkArm`))
                              (bind __piddata_2 (`/Game/Simulator/Multirotor/Blueprints/RollPitchControlExp.computeAngle` (`self.pitchValue`) (`self.trackYvar`) (`self.widgetYvar`) 5000.0 3.0 0.007 0.0 0.003 (`self.PlaneMesh`) (`self.pidYVar`)))
                              (set `self.pidYVar` __piddata_2)
                              (set `self.trackYvar` 0.0))))))))))))))
    (:`then_3`
      (if true
        ;[1 1 1] Animate Motors
        (`SceneComponent.K2_AddRelativeRotation` (`self.Motor1`) _returnvalue false false)
        (`SceneComponent.K2_AddRelativeRotation` (`self.Motor3`) _returnvalue false false)
        (`SceneComponent.K2_AddRelativeRotation` (`self.Motor2`) _returnvalue_2 false false)
        (`SceneComponent.K2_AddRelativeRotation` (`self.Motor4`) _returnvalue_2 false false)))
    (:`then_4`
      (if false
        (if (`self.closeLegs`)
          (if (< _returnvalue_5 90.0)
            (set `self.legPos` _returnvalue_5))
          (elif (!= _legpos 0.0)
            (set `self.legPos` (+ _legpos -2.0))))))
    (:`then_5`
      (if (!= (`self.legPos`) 0.0)
        ;[1 1 1] Animate Legs
        (`SceneComponent.K2_SetRelativeRotation` (`self.Leg1`) _returnvalue_4 false false)
        (`SceneComponent.K2_SetRelativeRotation` (`self.Leg2`) _returnvalue_4 false false)
        (`SceneComponent.K2_SetRelativeRotation` (`self.Leg3`) _returnvalue_4 false false)
        (`SceneComponent.K2_SetRelativeRotation` (`self.Leg4`) _returnvalue_4 false false)
        (`KismetSystemLibrary.PrintString` (`KismetStringLibrary.Conv_DoubleToString` (`self.legPos`)) true false (struct :`G` 0.66 :`B` 1.0 :`A` 1.0) 0.0)))
    (:`then_6`
      (if true
        (`SceneComponent.K2_SetRelativeRotation` (`self.gimbalBase`) (`KismetMathLibrary.MakeRotator` (* (.roll (`SceneComponent.K2_GetComponentRotation` (`self.PlaneMesh`))) -1.0) (* (.pitch (`SceneComponent.K2_GetComponentRotation` (`self.PlaneMesh`))) -1.0) 0.0) false false)))))

(event `InputAxis|Thrust`
  (params (AxisValue :type "Float (single-precision)"))
  ;[1 1 1] Car/Copter Control
  (set `self.curAxis` AxisValue))

(event `InputAxis|MoveUp`
  (params (AxisValue :type "Float (single-precision)"))
  ;[1 1 1] Car/Copter Control
  (set `self.pitchValue` AxisValue))

(event `InputAxis|MoveRight`
  (params (AxisValue :type "Float (single-precision)"))
  ;[1 1 1] Car/Copter Control
  (set `self.yawValue` AxisValue))

(event `InputAxis|Roll`
  (params (AxisValue :type "Float (single-precision)"))
  ;[1 1 1] Car/Copter Control
  (set `self.rollValue` AxisValue))

(event `InputAction|armUAV`
  (params (Key :type "Key Structure" :default "AnyKey"))
  ;[1 1 1] Car/Copter Control
  (:`Pressed`
    (set `self.ArmCopter` true)))

(event `Key|SpaceBar`
  (params (Key :type "Key Structure" :default "AnyKey"))
  ;[1 1 1] Car/Copter Control
  (:`Pressed`
    (`SimulatorFunctions.saveWayPoints` "C:/UnrealProjects/frames/uavTest.txt" (`|MakeArray` (13071.0 12575.0 22560.0) (15071.0 12575.0 22560.0) (14071.756836 11075.040039 22560.0) :!type "Vector Structure"))))

(event `Key|X`
  (params (Key :type "Key Structure" :default "AnyKey"))
  ;[1 1 1] Car/Copter Control
  (:`Pressed`
    (set `self.legPos` (+ (`self.legPos`) 1.0))))

(event `Key|S`
  (params (Key :type "Key Structure" :default "AnyKey"))
  ;[1 1 1] Car/Copter Control
  (:`Pressed`
    (set `self.legPos` (+ (`self.legPos`) -1.0))))

(fn `UserConstructionScript`)